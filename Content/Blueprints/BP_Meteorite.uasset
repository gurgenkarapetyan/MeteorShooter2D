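; BP_Meteorite is a 2D sprite meteorite that drifts and spins, awarding score and splitting into smaller meteorites when destroyed.
; SetMeteorite uses its size type to pick a random sprite, spin, direction and speed, with big ones aimed near world center and smaller ones faster.
; Tick moves it along that direction without sweeping.
; Destroy reports size-based points to the game mode, then big and medium rocks spawn two of the next size down.
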(event Custom|Set%20Meteorite
  (params (Type :type Enum_Meteorite_Type%20Enum :default "NewEnumerator0"))
  (bind _returnvalue (Math|Random|RandomFloatinRange -1.0 1.0))
  (bind _returnvalue_2 (Math|Random|RandomFloatinRange -1.0 1.0))
  (bind _returnvalue_3 (Math|Vector|MakeVector _returnvalue_2 0.0 _returnvalue))
  (bind _returnvalue_4 (Math|Vector|Normalize _returnvalue_3))
  ;[1 1 1] Set Meteorite
  (Variables|Default|SetType Type)
  (Variables|/Script/Engine.RotatingMovementComponent|SetRotationRate (Variables|Default|GetRotatingMovement) (Math|Rotator|MakeRotator 0.0 (Utilities|Select :Index (Math|Random|RandomInteger 3) :Option%200 -85.0 :Option%201 6e+01 :Option%202 -55.0 :Option%203 5e+01) 0.0))
  (bind _returnvalue_5 (AddComponent|AddPaperSpriteComponent false))
  (Rendering|Components|Sprite|SetSprite _returnvalue_5 (Utilities|Select :Index (Variables|Default|GetType) :NewEnumerator0 (Utilities|Select :Index (Math|Random|RandomIntegerinRange 0 3) :Option%200 "/Game/Sprites/meteorBrown_big1_Sprite.meteorBrown_big1_Sprite" :Option%201 "/Game/Sprites/meteorBrown_big2_Sprite.meteorBrown_big2_Sprite" :Option%202 "/Game/Sprites/meteorBrown_big3_Sprite.meteorBrown_big3_Sprite" :Option%203 "/Game/Sprites/meteorBrown_big4_Sprite.meteorBrown_big4_Sprite") :NewEnumerator1 (Utilities|Select :Index (Math|Random|RandomInteger 1) :Option%200 "/Game/Sprites/meteorBrown_med1_Sprite.meteorBrown_med1_Sprite" :Option%201 "/Game/Sprites/meteorBrown_med3_Sprite.meteorBrown_med3_Sprite") :NewEnumerator2 (Utilities|Select :Index (Math|Random|RandomInteger 1) :Option%200 "/Game/Sprites/meteorBrown_small1_Sprite.meteorBrown_small1_Sprite" :Option%201 "/Game/Sprites/meteorBrown_small2_Sprite.meteorBrown_small2_Sprite")))
  (Variables|Default|SetMoveDirection (Utilities|Select :Index (Variables|Default|GetType) :NewEnumerator0 (Math|Vector|Normalize (- (Math|Vector|MakeVector (Math|Random|RandomFloatinRange -3e+02 3e+02) 0.0 (Math|Random|RandomFloatinRange -8e+01 8e+01)) (Transformation|GetActorLocation))) :NewEnumerator1 _returnvalue_4 :NewEnumerator2 _returnvalue_4))
  (Variables|Default|SetSpeed (Utilities|Select :Index (Variables|Default|GetType) :NewEnumerator0 (Math|Random|RandomFloatinRange 6e+01 8e+01) :NewEnumerator1 (Math|Random|RandomFloatinRange 9e+01 1.1e+02) :NewEnumerator2 (Math|Random|RandomFloatinRange 1.2e+02 1.4e+02))))

(event Custom|Spawn%20New%20%28Meteorite%29
  (params (Type :type Enum_Meteorite_Type%20Enum :default "NewEnumerator0"))
  ;[1 1 1] Spawn New Meteorite
  (for _index (range 0 1)
    (bind _returnvalue (Game|SpawnActorfromClass "BP_Meteorite_C" (Math|Conversions|ToTransform(Vector) (Transformation|GetActorLocation)) "Undefined" 0 0))
    (Variables|BP_Meteorite_C|SetType _returnvalue Type)
    (CallFunction|SetMeteorite _returnvalue Type)))

(event Custom|Destroy
  (Class|BPActionsInterface|UpdateScore(Message) (Game|GetGameMode) (Utilities|Select :Index (Variables|Default|GetType) :NewEnumerator0 10 :NewEnumerator1 50 :NewEnumerator2 100))
  (switch Utilities|FlowControl|Switch|SwitchonEnum_Meteorite_Type (Variables|Default|GetType)
    (:NewEnumerator0
      (CallFunction|SpawnNew(Meteorite) "NewEnumerator1")
      (Actor|DestroyActor))
    (:NewEnumerator1
      (CallFunction|SpawnNew(Meteorite) "NewEnumerator2")
      (Actor|DestroyActor))
    (:NewEnumerator2
      (Actor|DestroyActor))))

(event EventTick
  (params (DeltaSeconds :type Float%20%28single-precision%29))
  ;[1 1 1] Move The Meteor In The Tick Event
  (Transformation|AddActorWorldOffset (* (Variables|Default|GetMoveDirection) (* DeltaSeconds (Variables|Default|GetSpeed)))))

(event EventBeginPlay
  ;[1 1 1] For TESTING PURPOSES ONLY
)

(fn ConstructionScript)