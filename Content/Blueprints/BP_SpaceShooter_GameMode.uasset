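; Game mode for a space shooter that runs meteorite waves, lives, score, HUD and best-score saving.
; BeginPlay creates the HUD, loads or creates the save, and starts a looping timer, its interval randomized once, for meteorite waves.
; Each wave spawns several meteorites at random preset angles around the Y axis.
; After a delay, player respawn deducts a life, then spawns a ship or triggers game over, saving any equal or higher score.
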(event Custom|Spawn%20Meteorite
  ;[1 1 1] Spawn Meteorite
  (Variables|Default|SetSpawn%20Points%20Temp (Variables|Default|GetSpawn%20Angles))
  (for _index (range 0 (Math|Random|RandomIntegerinRange 3 5))
    (Utilities|Array|Shuffle (Variables|Default|GetSpawn%20Points%20Temp))
    (bind _returnvalue (Game|SpawnActorfromClass "/Game/Blueprints/BP_Meteorite.BP_Meteorite_C" (Math|Transform|MakeTransform (Math|Vector|RotateVectorAroundAxis (Math|Vector|MakeVector (Variables|Default|GetX_Max) 0.0 (Variables|Default|GetZ_Max)) (Utilities|Array|Get(acopy) (Variables|Default|GetSpawn%20Points%20Temp) (Math|Random|RandomInteger (Utilities|Array|Length (Variables|Default|GetSpawn%20Points%20Temp)))) "0,1.000000, 0") "0, 0, 0" "1,1,1") "Undefined" 0 0))
    (Variables|/Game/Blueprints/BP_Meteorite.BP_Meteorite_C|SetType _returnvalue "NewEnumerator0")
    (Default|SetMeteorite _returnvalue "NewEnumerator0")))

(event Custom|Check%20Save%20Game%20Slot
  ;[1 1 1] Save Game
  (bind _returnvalue (SaveGame|DoesSaveGameExist (Variables|Default|GetSave%20Game%20Name)))
  (if _returnvalue
    (bind _returnvalue_2 (SaveGame|LoadGamefromSlot (Variables|Default|GetSave%20Game%20Name)))
    (bind _asbp_save_game (Utilities|Casting|CastToBP_SaveGame _returnvalue_2))
    (bind _output_get (Variables|Default|SetSave%20Game%20Instance%20REF _asbp_save_game))
    (Rendering|Components|TextRender|SetText (Variables|/Game/Blueprints/BP_Game_HUD.BP_Game_HUD_C|GetBestScoreValue (Variables|Default|GetGame%20HUD%20REF)) (Utilities|Text|ToText(Integer) (Variables|/Game/Blueprints/BP_SaveGame.BP_SaveGame_C|GetBest%20Score _output_get)))
    (else
      (bind _returnvalue_3 (SaveGame|CreateSaveGameObject "/Game/Blueprints/BP_SaveGame.BP_SaveGame_C"))
      (bind _output_get_2 (Variables|Default|SetSave%20Game%20Instance%20REF _returnvalue_3))
      (bind _output_get_3 (Variables|/Game/Blueprints/BP_SaveGame.BP_SaveGame_C|SetBest%20Score _output_get_2 0))
      (Rendering|Components|TextRender|SetText (Variables|/Game/Blueprints/BP_Game_HUD.BP_Game_HUD_C|GetBestScoreValue (Variables|Default|GetGame%20HUD%20REF)) (Utilities|Text|ToText(Integer) _output_get_3))
      (SaveGame|SaveGametoSlot _output_get_2 (Variables|Default|GetSave%20Game%20Name)))))

(event EventBeginPlay
  ;[1 1 1] Begin Play - Initialize
  (Variables|Default|SetLives 3)
  (Variables|Default|SetScore 0)
  (Variables|Default|SetSpawn%20Angles (Utilities|Array|MakeArray 0.0 6e+01 1.2e+02 1.8e+02 2.4e+02 3e+02))
  (CallFunction|SpawnMeteorite)
  (Utilities|Time|SetTimerbyFunctionName self "Spawn Meteorite" (Math|Random|RandomFloatinRange 6.0 1e+01) true)
  (bind _returnvalue (UserInterface|CreateWidget "/Game/Blueprints/BP_Game_HUD.BP_Game_HUD_C"))
  (bind _output_get (Variables|Default|SetGame%20HUD%20REF _returnvalue))
  (UserInterface|Viewport|AddtoViewport _output_get 0)
  (CallFunction|CheckSaveGameSlot))

(event EventTrytoSpawnPlayer
  ;[1 1 1] Try To Spawn Player
  (Utilities|FlowControl|Delay 1.0)
  (bind _output_get (Variables|Default|SetLives (- (Variables|Default|GetLives) 1)))
  (Default|UpdateLives (Variables|Default|GetGame%20HUD%20REF) _output_get)
  (Math|Integer|CompareInt (Variables|Default|GetLives) 0
    (:>
      (Game|SpawnActorfromClass "/Game/Blueprints/BP_SpaceShip.BP_SpaceShip_C" (Math|Transform|MakeTransform "0, 0, 0" "0, 0, 0" "1,1,1") "AdjustIfPossibleButDontSpawnIfColliding" 0 0))
    (:==
      (Default|GameOverEvent (Variables|Default|GetGame%20HUD%20REF))
      (bind _returnvalue (SaveGame|LoadGamefromSlot (Variables|Default|GetSave%20Game%20Name)))
      (bind _asbp_save_game (Utilities|Casting|CastToBP_SaveGame _returnvalue))
      (bind _output_get_2 (Variables|Default|SetSave%20Game%20Instance%20REF _asbp_save_game))
      (Math|Integer|CompareInt (Variables|/Game/Blueprints/BP_SaveGame.BP_SaveGame_C|GetBest%20Score _output_get_2) (Variables|Default|GetScore)
        (:==
          _)
        (:<
          _))
      (bind _output_get_3 (Variables|/Game/Blueprints/BP_SaveGame.BP_SaveGame_C|SetBest%20Score (Variables|Default|GetSave%20Game%20Instance%20REF) (Variables|Default|GetScore)))
      (Rendering|Components|TextRender|SetText (Variables|/Game/Blueprints/BP_Game_HUD.BP_Game_HUD_C|GetBestScoreValue (Variables|Default|GetGame%20HUD%20REF)) (Utilities|Text|ToText(Integer) _output_get_3))
      (SaveGame|SaveGametoSlot (Variables|Default|GetSave%20Game%20Instance%20REF) (Variables|Default|GetSave%20Game%20Name)))))

(event EventUpdateScore
  (params (Value :type Integer))
  ;[1 1 1] Update Score
  (Variables|Default|SetScore (+ Value (Variables|Default|GetScore)))
  (Rendering|Components|TextRender|SetText (Variables|/Game/Blueprints/BP_Game_HUD.BP_Game_HUD_C|GetScoreValue (Variables|Default|GetGame%20HUD%20REF)) (Utilities|Text|ToText(Integer) (Variables|Default|GetScore))))

(fn ConstructionScript)